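; Health component that tracks its owner's health and shows it through a health bar widget created and added to the viewport on BeginPlay.
; AddHealth subtracts InDamage, so negative values heal, clamps the result between zero and MaxHealth, then has the widget refresh.
; A pickup or punch sound with random pitch plays at the owner's location, except when health gets capped at maximum.
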(event EventBeginPlay
  (bind _returnvalue (UserInterface|CreateWidget "/Game/TestFiles/Blueprints/Widgets/Health/UW_HealthBar.UW_HealthBar_C" 0 self))
  (UserInterface|Viewport|AddtoViewport _returnvalue 0)
  (Variables|Default|SetUW_HealthBar _returnvalue))

(event EventTick
  (params (DeltaSeconds :type Float%20%28single-precision%29)))

(fn OnHealthChange
  (Utilities|FlowControl|Sequence
    (:then_0
      (Default|UpdateHealth (Variables|Default|GetUW_HealthBar)))))

(fn AddHealth
  (params (InDamage :type Integer))
  (Utilities|FlowControl|Sequence
    (:then_0
      (LocalVariables|SetLocal_ChangedHealth (- (Variables|Default|GetCurrentHealth) InDamage))
      (if (< (LocalVariables|GetLocal_ChangedHealth) 0)
        (Variables|Default|SetCurrentHealth 0)
        (CallFunction|PlaySound InDamage :!label _label)
        (elif (> (LocalVariables|GetLocal_ChangedHealth) (Variables|Default|GetMaxHealth))
          (Variables|Default|SetCurrentHealth (Variables|Default|GetMaxHealth))
          (else
            (Variables|Default|SetCurrentHealth (LocalVariables|GetLocal_ChangedHealth))
            (goto _label)))))
    (:then_1
      (CallFunction|OnHealthChange))))

(fn PlaySound
  (params (InDamage :type Integer))
  (if (< InDamage 0)
    (Audio|PlaySoundatLocation "/Game/TestFiles/Audio/health-pickup.health-pickup" (Transformation|GetActorLocation (Components|GetOwner)) "0, 0, 0" 1.0 (Math|Random|RandomFloatinRange 0.4 1.0) 0.0 0 0 0 0)
    (else
      (Audio|PlaySoundatLocation "/Game/TestFiles/Audio/major-punch.major-punch" (Transformation|GetActorLocation (Components|GetOwner)) "0, 0, 0" 1.0 (Math|Random|RandomFloatinRange 0.4 1.0) 0.0 0 0 0 0))))