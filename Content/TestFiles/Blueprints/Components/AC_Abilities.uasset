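; Actor component that gives its owner a dash ability through the Gameplay Ability System.
; On BeginPlay it caches the owner's AbilitySystemComponent, adding one at runtime if none exists, then grants the dash ability to it.
; The TryDash event activates that ability by class, with remote activation allowed.
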(event Custom|TryDash
  (Abilities|TryActivateAbilitybyClass (Variables|Default|GetAbilitySystem) (Variables|Default|GetDashAbility) true))

(event EventBeginPlay
  (bind _returnvalue (Components|GetOwner))
  (bind _returnvalue_2 (Actor|GetComponentbyClass _returnvalue "/Script/GameplayAbilities.AbilitySystemComponent"))
  (Utilities|FlowControl|Sequence
    (:then_0
      (Utilities|IsValid _returnvalue_2
        (:Is%20Valid
          (Variables|Default|SetAbilitySystem _returnvalue_2))
        (:Is%20Not%20Valid
          (bind _returnvalue_3 (Game|AddComponentbyClass (Components|GetOwner) "/Script/GameplayAbilities.AbilitySystemComponent"))
          (Variables|Default|SetAbilitySystem _returnvalue_3))))
    (:then_1
      (Utilities|IsValid (Variables|Default|GetAbilitySystem)
        (:Is%20Valid
          (GameplayAbilities|GiveAbility (Variables|Default|GetAbilitySystem) (Variables|Default|GetDashAbility) 0 -1))))))

(event EventTick
  (params (DeltaSeconds :type Float%20%28single-precision%29)))